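; Test first-person character that prototypes camera recoil for automatic fire, with mouse look.
; Holding left mouse loops a Fire timer that banks interpolated kick into accumulated recoil.
; Tick rebuilds camera pitch and capsule yaw from PlayerRotation, layering recoil on top via FInterpTo, then decaying it after release.
; Downward mouse movement while firing is tracked to offset recoil, so recovery doesn't snap below the starting aim point.
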(event `Fire`
  ;[1 0.5103 0.934] Case 1: Accumulation occurs when firing again
  (set `self.AccumulatedRecoil` (+ (`self.AccumulatedRecoil`) (`self.InterpRecoil`)))
  (set `self.InterpRecoil` 0.0)
  (set `self.bInterpingRecoil` true))

(event `Key|LeftMouseButton`
  (params (Key :type "Key Structure"))
  (bind (_playerrotation_roll _playerrotation_pitch _playerrotation_yaw) (`KismetMathLibrary.BreakRotator` (`self.PlayerRotation`)))
  (:`Pressed`
    (if (not (`self.bInterpingRecoil`))
      (set `self.PlayerRotation` (`KismetMathLibrary.MakeRotator` _playerrotation_roll (+ _playerrotation_pitch (`self.AmountPulledDown`)) _playerrotation_yaw))
      (set `self.AmountPulledDown` 0.0))
    (`self.Fire`)
    (set `self.bIsFiring` true)
    (bind _returnvalue (`KismetSystemLibrary.K2_SetTimerDelegate` (delegate `Fire`) 0.1 true))
    (set `self.FireHandle` _returnvalue))
  (:`Released`
    (`KismetSystemLibrary.K2_ClearAndInvalidateTimerHandle` (`self.FireHandle`))
    (set `self.bIsFiring` false)))

(event `InputAxisKey|MouseX`
  (params (AxisValue :type "Float (single-precision)"))
  (bind (_playerrotation_roll _playerrotation_pitch _playerrotation_yaw) (`KismetMathLibrary.BreakRotator` (`self.PlayerRotation`)))
  (set `self.PlayerRotation` (`KismetMathLibrary.MakeRotator` _playerrotation_roll _playerrotation_pitch (+ _playerrotation_yaw AxisValue))))

(event `InputAxisKey|MouseY`
  (params (AxisValue :type "Float (single-precision)"))
  (bind (_playerrotation_roll _playerrotation_pitch _playerrotation_yaw) (`KismetMathLibrary.BreakRotator` (`self.PlayerRotation`)))
  ;[1 1 1] Pulling Down?
  (if (and (< AxisValue 0.0) (`self.bIsFiring`))
    (set `self.AmountPulledDown` (- (`self.AmountPulledDown`) AxisValue)))
  (set `self.PlayerRotation` (`KismetMathLibrary.MakeRotator` _playerrotation_roll (+ _playerrotation_pitch AxisValue) _playerrotation_yaw)))

(event `self.ReceiveTick`
  (params (DeltaSeconds :type "Float (single-precision)"))
  (bind (_playerrotation_roll _playerrotation_pitch _playerrotation_yaw) (`KismetMathLibrary.BreakRotator` (`self.PlayerRotation`)))
  (bind (_playerrotation_roll_2 _playerrotation_pitch_2 _playerrotation_yaw_2) (`KismetMathLibrary.BreakRotator` (`self.PlayerRotation`)))
  (bind (_playerrotation_roll_3 _playerrotation_pitch_3) (`KismetMathLibrary.BreakRotator` (`self.PlayerRotation`)))
  (bind (_playerrotation_roll_4 _playerrotation_pitch_4 _playerrotation_yaw_3) (`KismetMathLibrary.BreakRotator` (`self.PlayerRotation`)))
  (`SceneComponent.K2_SetRelativeRotation` (`self.Camera`) (`KismetMathLibrary.MakeRotator` 0.0 _playerrotation_pitch) false false)
  (`SceneComponent.K2_SetWorldRotation` (`self.CapsuleComponent`) (`KismetMathLibrary.MakeRotator` 0.0 0.0 _playerrotation_yaw) false false)
  (if (`self.bInterpingRecoil`)
    (set `self.InterpRecoil` (`KismetMathLibrary.FInterpTo` (`self.InterpRecoil`) (`self.TargetInterpRecoil`) DeltaSeconds (`self.InterpSpeed`)))
    (if (>= (`self.InterpRecoil`) (* (`self.TargetInterpRecoil`) 0.98))
      (set `self.bInterpingRecoil` false)
      ;[1 0.3471 0.7164] Case 2: Accumulation occurs when interp is finished
      (set `self.AccumulatedRecoil` (+ (`self.AccumulatedRecoil`) (`self.TargetInterpRecoil`)))
      (set `self.InterpRecoil` 0.0)
      (if (< (`self.AmountPulledDown`) (`self.AccumulatedRecoil`))
        (set `self.AccumulatedRecoil` (- (`self.AccumulatedRecoil`) (`self.AmountPulledDown`)))
        (`SceneComponent.K2_AddRelativeRotation` (`self.Camera`) (`KismetMathLibrary.MakeRotator` 0.0 (+ (`self.AccumulatedRecoil`) (`self.AmountPulledDown`))) false false)
        (else
          (set `self.PlayerRotation` (`KismetMathLibrary.MakeRotator` _playerrotation_roll_4 (+ _playerrotation_pitch_4 (`self.AccumulatedRecoil`)) _playerrotation_yaw_3))
          ;[1 1 1] Duplicate call avoids single frame of incorrect look. Poor optimization but oh well
          (`SceneComponent.K2_SetRelativeRotation` (`self.Camera`) (`KismetMathLibrary.MakeRotator` 0.0 _playerrotation_pitch_3) false false)
          (set `self.AccumulatedRecoil` 0.0)
          (set `self.AmountPulledDown` 0.0)))
      (else
        ;[1 1 1] Addition of Interp and Accum hasn't occured yet. Must be done frame by frame
        (`SceneComponent.K2_AddRelativeRotation` (`self.Camera`) (`KismetMathLibrary.MakeRotator` 0.0 (+ (`self.AccumulatedRecoil`) (`self.InterpRecoil`))) false false)))
    (elif (and (> (`self.AccumulatedRecoil`) 0.0) (not (`self.bIsFiring`)))
      ;[1 1 1] Decaying
      (bind _output_get (set `self.AccumulatedRecoil` (- (`self.AccumulatedRecoil`) 0.3)))
      (if (< _output_get 0.0)
        ;[1 1 1] Adding offset so crosshair doesn't snap back below point where firing began
        (set `self.PlayerRotation` (`KismetMathLibrary.MakeRotator` _playerrotation_roll_2 (+ _playerrotation_pitch_2 (`self.AmountPulledDown`)) _playerrotation_yaw_2))
        ;;[1 1 1] Still needed for this frame
        (`SceneComponent.K2_AddRelativeRotation` (`self.Camera`) (`KismetMathLibrary.MakeRotator` 0.0 (`self.AmountPulledDown`)) false false)
        (set `self.AmountPulledDown` 0.0)
        (set `self.AccumulatedRecoil` 0.0)
        (else
          (`SceneComponent.K2_AddRelativeRotation` (`self.Camera`) (`KismetMathLibrary.MakeRotator` 0.0 (+ (`self.AccumulatedRecoil`) (`self.AmountPulledDown`))) false false))))))

(fn `UserConstructionScript`)