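; BP_Grenade is a test-enemy grenade actor that explodes on a short timer after spawning.
; On explosion it plays a particle effect and runs a stationary multi-sphere trace on the Visibility channel at its location.
; Each hit that casts to GameCharacter receives fixed Fire damage, with debug prints for cast results, then the grenade destroys itself.
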(event `self.ReceiveBeginPlay`
  (`KismetSystemLibrary.K2_SetTimerDelegate` (delegate `Event Explose`) 1.5))

(event `Event Explose`
  (bind _returnvalue (`self.K2_GetActorLocation`))
  (`GameplayStatics.SpawnEmitterAtLocation` "/Game/Assets/MilitaryWeapDark/FX/P_Grenade_Explosion_01.P_Grenade_Explosion_01" (`self.K2_GetActorLocation`))
  (bind _outhits (`KismetSystemLibrary.SphereTraceMulti` _returnvalue _returnvalue 500.0 "TraceTypeQuery1"))
  (for _array_element _outhits
    (bind _asgame_character (cast `GameCharacter` (`.HitActor` (`GameplayStatics.BreakHitResult` _array_element)))
      (:`then`
        (`KismetSystemLibrary.PrintString` "Hello")
        (`GameCharacter.ReceiveDamage` _asgame_character (make `DamageStruct` 30.0 "EDT_Fire")))
      (:`CastFailed`
        (`KismetSystemLibrary.PrintString` "CastFailed"))))
  (`self.K2_DestroyActor`))

(fn `UserConstructionScript`)