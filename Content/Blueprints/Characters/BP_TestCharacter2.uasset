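; Test character that prototypes accumulating camera recoil with recovery, driven by mouse look and held left-click automatic fire.
; A looping timer calls Fire, which banks any partial kick and starts a new eased one that Tick advances.
; Tick layers recoil pitch over a separately clamped player rotation, split between camera pitch and capsule yaw.
; Between kicks, recoil decays until it reaches StoredPitch, which tracks positive pitch input, then folds the remainder into player rotation.
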(event `Fire`
  ;[1 0.5103 0.934] Case 1: Accumulation occurs when firing again
  (set `self.AccumulatedRecoil` (+ (`self.AccumulatedRecoil`) (`self.InterpRecoil`)))
  (set `self.InterpRecoil` 0.0)
  (set `self.bInterpingRecoil` true))

(event `Key|LeftMouseButton`
  (params (Key :type "Key Structure"))
  (:`Pressed`
    (`self.Fire`)
    (set `self.bIsFiring` true)
    (bind _returnvalue (`KismetSystemLibrary.K2_SetTimerDelegate` (delegate `Fire`) 0.1 true))
    (set `self.FireHandle` _returnvalue))
  (:`Released`
    (`KismetSystemLibrary.K2_ClearAndInvalidateTimerHandle` (`self.FireHandle`))
    (set `self.bIsFiring` false)))

(event `InputAxis|LookRight`
  (params (AxisValue :type "Float (single-precision)"))
  (`self.AddPlayerRotation` 0.0 AxisValue))

(event `InputAxis|LookUp`
  (params (AxisValue :type "Float (single-precision)"))
  (bind _returnvalue (* -1 AxisValue))
  (`self.AddPlayerRotation` _returnvalue
    (:`Out`
      (if (> _returnvalue 0.0)
        (set `self.StoredPitch` (+ (`self.StoredPitch`) _returnvalue))))))

(event `self.ReceiveTick`
  (params (DeltaSeconds :type "Float (single-precision)"))
  (bind (_playerrotation_roll _playerrotation_pitch) (`KismetMathLibrary.BreakRotator` (`self.PlayerRotation`)))
  (bind (_playerrotation_roll_2 _playerrotation_pitch_2 _playerrotation_yaw) (`KismetMathLibrary.BreakRotator` (`self.PlayerRotation`)))
  (`SceneComponent.K2_SetRelativeRotation` (`self.Camera`) (`KismetMathLibrary.MakeRotator` 0.0 _playerrotation_pitch_2) false false)
  (`SceneComponent.K2_SetWorldRotation` (`self.CapsuleComponent`) (`KismetMathLibrary.MakeRotator` 0.0 0.0 _playerrotation_yaw) false false)
  (if (`self.bInterpingRecoil`)
    (set `self.InterpRecoil` (`KismetMathLibrary.FInterpEaseInOut` (`self.InterpRecoil`) (`self.TargetInterpRecoil`) DeltaSeconds 0.2))
    (if (>= (`self.InterpRecoil`) (* (`self.TargetInterpRecoil`) 0.98))
      (set `self.bInterpingRecoil` false)
      ;[1 0.3471 0.7164] Case 2: Accumulation occurs when interp is finished
      (set `self.AccumulatedRecoil` (+ (`self.AccumulatedRecoil`) (`self.TargetInterpRecoil`)))
      (set `self.InterpRecoil` 0.0)
      (`SceneComponent.K2_AddRelativeRotation` (`self.Camera`) (`KismetMathLibrary.MakeRotator` 0.0 (`self.AccumulatedRecoil`)) false false)
      (else
        ;[1 1 1] Addition of Interp and Accum hasn't occured yet. Must be done frame by frame
        (`SceneComponent.K2_AddRelativeRotation` (`self.Camera`) (`KismetMathLibrary.MakeRotator` 0.0 (+ (`self.AccumulatedRecoil`) (`self.InterpRecoil`))) false false)))
    (elif (<= (+ (`self.AccumulatedRecoil`) _playerrotation_pitch) (`self.StoredPitch`))
      ;[1 1 1] Past the stored firing angle. Setting player rotation for next frame and adding for this one
      (`self.AddPlayerRotation` (`self.AccumulatedRecoil`)
        (:`Out`
          (`SceneComponent.K2_AddRelativeRotation` (`self.Camera`) (`KismetMathLibrary.MakeRotator` 0.0 (`self.AccumulatedRecoil`)) false false)
          (set `self.AccumulatedRecoil` 0.0)))
      (else
        (set `self.AccumulatedRecoil` (- (`self.AccumulatedRecoil`) 0.3))
        (`SceneComponent.K2_AddRelativeRotation` (`self.Camera`) (`KismetMathLibrary.MakeRotator` 0.0 (`self.AccumulatedRecoil`)) false false)))))

(fn `UserConstructionScript`)