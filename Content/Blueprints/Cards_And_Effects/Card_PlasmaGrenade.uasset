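; Card effect that spawns a PlasmaGrenade when the card is used.
; Use takes the spawn location and rotation from MakeTransform, then sets the player character as the grenade's GameCharacter.
; The MakeTransform graph holds math for a point just ahead of the player's eye view point, facing the view direction, though that node is shown as unused.
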(event EventUse
  (bind _returnvalue (Math|Transform|MakeTransform))
  (bind _returnvalue_2 (Class|Card|SpawnActor "/Game/Blueprints/Cards_And_Effects/CardSpawnedActors/PlasmaGrenade.PlasmaGrenade_C" (.rotation _returnvalue) (.location _returnvalue)))
  (bind _asplasma_grenade (Utilities|Casting|CastToPlasmaGrenade _returnvalue_2))
  (Variables|/Game/Blueprints/Cards_And_Effects/CardSpawnedActors/PlasmaGrenade.PlasmaGrenade_C|SetGameCharacter _asplasma_grenade (Variables|Default|GetPlayerCharacter)))