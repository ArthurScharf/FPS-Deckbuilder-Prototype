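; Card_TEST is a test card that applies the SE_TEST status effect to the player character when used.
; Its spawned-actor callback deals Fire damage to the passed game character, crediting the player as the damage causer.
; A disconnected node would spawn a bullet projectile just ahead of the player, but it never runs, so Use itself spawns nothing.
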(event `self.Use`
  (`GameCharacter.InstantiateStatusEffect` (`self.PlayerCharacter`) "/Game/Blueprints/StatusEffects/SE_TEST.SE_TEST_C"))

(event `self.SpawnedActorCallback`
  (params (GameCharacter :type "GameCharacter Object Reference") (Location :type "Vector Structure"))
  (`GameCharacter.ReceiveDamage` GameCharacter (make `DamageStruct` (`self.Damage`) "EDT_Fire" (0.0 0.0 0.0) (`self.PlayerCharacter`))))