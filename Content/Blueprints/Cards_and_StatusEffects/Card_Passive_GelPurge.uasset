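; Passive card that turns heavy poison on a damaged character into a spreading burst.
; It observes the player's damage-dealt notifications, and when the receiver's SE_Poison stacks reach a threshold, it cleans up that effect.
; A sphere overlap then finds nearby GameCharacters, excluding the receiver, and gives each extra poison stacks instigated by the player.
; A HasTriggered guard blocks re-entry, since applying poison re-fires the notification and would loop infinitely.
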(event `self.Subscribe`
  (`GameCharacter.AddObserver_OnDamageDealt` (`self.PlayerCharacter`) (`|CreateDelegate` :!event `HandleNotify`)))

(event `self.Unsubscribe`
  (`GameCharacter.RemoveObserver_OnDamageDealt` (`self.PlayerCharacter`) (`|CreateDelegate` :!event `HandleNotify`)))

(fn `HandleNotify`
  (params (DamageStruct :type "DamageStruct Structure (by ref)"))
  (locals (AffectedGameCharacter :type "GameCharacter Object Reference"))
  (if (not (`self.bHasTriggered`))
    (set `self.bHasTriggered` true)
    (bind _output_get (set `local.AffectedGameCharacter` (`.DamageReceiver` (break `DamageStruct` DamageStruct))))
    (for _array_element (`GameCharacter.StatusEffects` _output_get)
      (if (== (`GameplayStatics.GetObjectClass` _array_element) "/Game/Blueprints/Cards_and_StatusEffects/StatusEffects/SE_Poison.SE_Poison_C")
        (if (>= (`StatusEffect.NumInstances` _array_element) 6)
          (`StatusEffect.Cleanup` _array_element)
          (bind _outactors (`self.SphereOverlapActors` (`Actor.K2_GetActorLocation` (`local.AffectedGameCharacter`)) 300.0 (`|MakeArray` "ObjectTypeQuery8" "ObjectTypeQuery7" :!type "EObjectTypeQuery Enum") "/Script/FPS_Deckbuilder.GameCharacter" (`|MakeArray` (`local.AffectedGameCharacter`) :!type "Actor Object Reference") true))
          (for _array_element_2 _outactors
            (bind _asgame_character (cast `GameCharacter` _array_element_2))
            (bind _returnvalue (`GameCharacter.InstantiateStatusEffect` _asgame_character "/Game/Blueprints/Cards_and_StatusEffects/StatusEffects/SE_Poison.SE_Poison_C" (`self.PlayerCharacter`)))
            (set `StatusEffect.NumInstances` (+ (`StatusEffect.NumInstances` _returnvalue) 4) _returnvalue)))))
    ;[1 1 1] Instantiating more poison will trigger this entire method. Having this set at the beginning of the first call of this method and only unsetting it once the method is done being called avoids an infinite loop
    (set `self.bHasTriggered` false)
    (return)))