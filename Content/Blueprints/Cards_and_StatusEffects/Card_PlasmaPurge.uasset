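; Plasma Purge card Blueprint that rotates a player's card stack whose selected card is a Plasma Block.
; CanUse extends the parent check by asking the player character for such a stack and passes only if one is found.
; The lookup caches the result in RotatableSlot as a side effect, which Use then rotates and clears.
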(event `self.Use`
  (`TrayStack.Rotate` (`self.RotatableSlot`))
  (set `self.RotatableSlot` null))

(fn `CanUse`
  (returns (ReturnValue :type Boolean))
  (bind _returnvalue (`parent.CanUse`))
  (if _returnvalue
    (bind _returnvalue_2 (`PlayerCharacter.GetStackWithSelectedCardOfClass` (`self.PlayerCharacter`) "/Game/Blueprints/Cards_and_StatusEffects/BlockingCards/Card_PlasmaBlock.Card_PlasmaBlock_C"))
    (bind _output_get (set `self.RotatableSlot` _returnvalue_2))
    (if (!= _output_get null)
      (return true)
      (else
        (return false)))))