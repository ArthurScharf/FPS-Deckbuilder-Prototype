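; Warlord card Blueprint that accumulates the damage the player deals and, when used, applies the Warlord status effect to the player.
; Subscribe and Unsubscribe add and remove an observer on the player character's damage-dealt notifications.
; HandleNotify adds each hit's damage to a stored total, capped at a maximum.
; Use instantiates SE_Warlord with the player as instigator and always succeeds, without reading or resetting the stored total.
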(event `self.Subscribe`
  (`GameCharacter.AddObserver_OnDamageDealt` (`self.PlayerCharacter`) (`|CreateDelegate` :!event `HandleNotify`)))

(event `self.Unsubscribe`
  (`GameCharacter.RemoveObserver_OnDamageDealt` (`self.PlayerCharacter`) (`|CreateDelegate` :!event `HandleNotify`)))

(fn `HandleNotify`
  (params (DamageStruct :type "DamageStruct Structure (by ref)"))
  (set `self.DamageStored` (+ (`.Damage` (break `DamageStruct` DamageStruct)) (`self.DamageStored`)))
  (if (> (`self.DamageStored`) (`self.DamageStoredMax`))
    (set `self.DamageStored` (`self.DamageStoredMax`)))
  (return))

(fn `Use`
  (returns (ReturnValue :type Boolean))
  (bind _playercharacter (`self.PlayerCharacter`))
  (`GameCharacter.InstantiateStatusEffect` _playercharacter "/Game/Blueprints/Cards_and_StatusEffects/StatusEffects/SE_Warlord.SE_Warlord_C" _playercharacter)
  (return true))