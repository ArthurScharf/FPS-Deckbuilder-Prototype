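; Shadow Strike card ability that teleports the player to an aimed point and stuns enemies around the landing spot.
; On use, a Visibility line trace runs from the camera to a far point built from the view rotation, without adding the camera location.
; On a blocking hit, the player teleports to the impact point without sweeping.
; A sphere overlap there then briefly stuns each EnemyCharacter found.
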(event `self.Use`
  (bind (_outlocation _outrotation) (`PlayerCharacter.GetCameraViewPoint` (`self.PlayerCharacter`)))
  (bind (_bblockinghit _binitialoverlap _time _distance _location _impactpoint) (`GameplayStatics.BreakHitResult` (`self.LineTraceSingleByChannel` _outlocation (`KismetMathLibrary.GreaterGreater_VectorRotator` (`KismetMathLibrary.MakeVector` 10000.0) _outrotation) "ECC_Visibility" (`|MakeArray` null :!type "Actor Object Reference") true)))
  (if _bblockinghit
    (`Actor.K2_SetActorLocation` (`self.PlayerCharacter`) _impactpoint false true)
    (bind _outactors (`self.SphereOverlapActors` _impactpoint 500.0 (`|MakeArray` "ObjectTypeQuery8" :!type "EObjectTypeQuery Enum") "/Script/FPS_Deckbuilder.EnemyCharacter" (`|MakeArray` null :!type "Actor Object Reference") true))
    (for _array_element _outactors
      (bind _asenemy_character (cast `EnemyCharacter` _array_element))
      (`GameCharacter.Stun` _asenemy_character 1.2))))