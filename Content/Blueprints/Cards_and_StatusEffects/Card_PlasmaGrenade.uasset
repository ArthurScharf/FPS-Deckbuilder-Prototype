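; A card that throws a plasma grenade and places a companion Plasma Block card in the player's card stack.
; Modifying the stack constructs the block card, sets it in the leading empty slot and refreshes the stack editor; reverting removes that same card.
; Use spawns a PlasmaGrenade just ahead of the player's eye viewpoint and assigns the player as its GameCharacter, reporting failure if the cast fails.
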(fn `ModifyStack`
  (params (Stack :type "TrayStack Object Reference"))
  (returns (ReturnValue :type Boolean))
  (bind _returnvalue (`|GenericCreateObject` "/Game/Blueprints/Cards_and_StatusEffects/BlockingCards/Card_PlasmaBlock.Card_PlasmaBlock_C" self))
  (set `self.ManagedBlock` _returnvalue)
  (bind _returnvalue_2 (`TrayStack.GetLeadingEmptySlot` Stack))
  (set `self.ModifiedSlot` _returnvalue_2)
  (bind _returnvalue_3 (`TrayStack.SetCardInSlot` Stack _returnvalue_2 0 (`self.ManagedBlock`)))
  (`PlayerCharacter.UpdateStackEditor` (`self.PlayerCharacter`))
  (return _returnvalue_3))

(fn `RevertModifyStack`
  (params (Stack :type "TrayStack Object Reference"))
  (returns (ReturnValue :type Boolean))
  (bind _returnvalue (`TrayStack.RemoveCard` Stack (`self.ManagedBlock`)))
  (`PlayerCharacter.UpdateStackEditor` (`self.PlayerCharacter`))
  (return _returnvalue))

(fn `Use`
  (returns (ReturnValue :type Boolean))
  (bind (_outlocation _outrotation) (`Actor.GetActorEyesViewPoint` (`self.PlayerCharacter`)))
  (bind _returnvalue (`self.SpawnActor` "/Game/Blueprints/Cards_and_StatusEffects/CardSpawnedActors/PlasmaGrenade.PlasmaGrenade_C" (.rotation (`KismetMathLibrary.MakeTransform` (+ _outlocation (`KismetMathLibrary.GreaterGreater_VectorRotator` (`KismetMathLibrary.MakeVector` 100.0) _outrotation)) _outrotation (1.0 1.0 1.0))) (.location (`KismetMathLibrary.MakeTransform` (+ _outlocation (`KismetMathLibrary.GreaterGreater_VectorRotator` (`KismetMathLibrary.MakeVector` 100.0) _outrotation)) _outrotation (1.0 1.0 1.0)))))
  (bind _asplasma_grenade (cast `/Game/Blueprints/Cards_and_StatusEffects/CardSpawnedActors/PlasmaGrenade` _returnvalue)
    (:`then`
      (set `/Game/Blueprints/Cards_and_StatusEffects/CardSpawnedActors/PlasmaGrenade.GameCharacter` (`self.PlayerCharacter`) _asplasma_grenade)
      (return true))
    (:`CastFailed`
      (`KismetSystemLibrary.PrintString` null "UCard::Use -- Failed to spawn grenade")
      (return false))))