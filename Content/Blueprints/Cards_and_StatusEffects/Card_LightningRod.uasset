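; Lightning Rod card that fires a rod projectile from the player's view point, damaging and applying a status effect to the character it hits.
; On use, it spawns the projectile without collision, binds its overlap notify, then enables collision.
; On overlap, the rod attaches to the target's mesh, deals damage that can trigger status effects, and instantiates SE_LightningRod with the player as instigator.
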(event `self.Use`
  (bind _playercharacter (`self.PlayerCharacter`))
  (bind (_outlocation _outrotation) (`Actor.GetActorEyesViewPoint` _playercharacter))
  (bind _returnvalue (`GameCharacter.SpawnProjectileWithoutCollision` _playercharacter "/Game/Blueprints/Cards_and_StatusEffects/CardSpawnedActors/Projectile_LightningRod.Projectile_LightningRod_C" (`KismetMathLibrary.MakeTransform` (+ _outlocation (`KismetMathLibrary.GreaterGreater_VectorRotator` (`KismetMathLibrary.MakeVector` 100.0) _outrotation)) _outrotation)))
  (bind _asprojectile_lightning_rod (cast `/Game/Blueprints/Cards_and_StatusEffects/CardSpawnedActors/Projectile_LightningRod` _returnvalue))
  (bind _output_get (set `self.LightningRod` _asprojectile_lightning_rod))
  (add `Projectile.OnBeginOverlapNotify` _returnvalue (delegate `ApplyDamage`))
  (`Actor.SetActorEnableCollision` _output_get true))

(event `ApplyDamage`
  (params (HitGameCharacter :type "GameCharacter Object Reference") (HitResult :type "HitResult Structure (by ref)"))
  (`Actor.K2_AttachToComponent` (`self.LightningRod`) (`Character.Mesh` HitGameCharacter) "None" "KeepWorld" "KeepWorld" "KeepWorld" true)
  (`GameCharacter.ReceiveDamage` HitGameCharacter (make `DamageStruct` 5.0 "EDT_Physical" (0.0 0.0 0.0) (`self.PlayerCharacter`) null "None" false false HitResult) true)
  (`GameCharacter.InstantiateStatusEffect` HitGameCharacter "/Game/Blueprints/Cards_and_StatusEffects/StatusEffects/SE_LightningRod.SE_LightningRod_C" (`self.PlayerCharacter`)))