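; Lightning rod card that, on use, spawns a Projectile_LightningRod from the player character.
; It binds the projectile's begin-overlap notify to ApplyDamage, then enables collision on the LightningRod reference.
; Despite its name, ApplyDamage only spawns a StaticMeshActor at the rod's transform and calls SetStaticMesh without a mesh.
; The damage and attach-to-target nodes are disconnected, and MakeTransform's eye-view offset calculation is unused.
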(event `self.Use`
  (bind _playercharacter (`self.PlayerCharacter`))
  (bind (_outlocation _outrotation) (`Actor.GetActorEyesViewPoint` _playercharacter))
  (bind _returnvalue (`GameCharacter.SpawnProjectileWithoutCollision` _playercharacter "/Game/Blueprints/Cards/CardSpawnedActors/Projectile_LightningRod.Projectile_LightningRod_C" (`KismetMathLibrary.MakeTransform` (+ _outlocation (`KismetMathLibrary.GreaterGreater_VectorRotator` (`KismetMathLibrary.MakeVector` 100.0) _outrotation)) _outrotation)))
  (bind _output_get (set `self.LightningRod` null))
  (add `Projectile.OnBeginOverlapNotify` _returnvalue (delegate `ApplyDamage`))
  (`Actor.SetActorEnableCollision` _output_get true))

(event `ApplyDamage`
  (params (HitGameCharacter :type "GameCharacter Object Reference") (HitResult :type "HitResult Structure (by ref)"))
  (bind _lightningrod (`self.LightningRod`))
  (bind _returnvalue (`self.SpawnActor` "/Script/Engine.StaticMeshActor" (`Actor.K2_GetActorRotation` _lightningrod) (`Actor.K2_GetActorLocation` _lightningrod)))
  (bind _asstatic_mesh_actor (cast `StaticMeshActor` _returnvalue))
  (`StaticMeshComponent.SetStaticMesh` (`StaticMeshActor.StaticMeshComponent` _asstatic_mesh_actor) null))